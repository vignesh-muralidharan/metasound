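; BP_SongSwitcher is a trigger-volume actor that switches the playing song while something is inside its Box.
; On BeginPlay it caches the first BP_AudioPlayer found in the level.
; Box begin and end overlap set the integer SongValue parameter on that actor's Player component to 1 and 0, with no filtering of the overlapping actor.
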(event `self.ReceiveBeginPlay`
  (bind _outactors (`GameplayStatics.GetAllActorsOfClass` "/Game/Blueprints/BP_AudioPlayer.BP_AudioPlayer_C"))
  (set `self.AudioPlayerReference` (`|GetArrayItem` _outactors)))

(event `self.Box.OnComponentBeginOverlap`
  (params (OverlappedComponent :type "PrimitiveComponent Object Reference") (OtherActor :type "Actor Object Reference") (OtherComp :type "PrimitiveComponent Object Reference") (OtherBodyIndex :type Integer) (bFromSweep :type Boolean) (SweepResult :type "HitResult Structure (by ref)"))
  (`AudioComponent.SetIntParameter` (`/Game/Blueprints/BP_AudioPlayer.Player` (`self.AudioPlayerReference`)) "SongValue" 1))

(event `self.Box.OnComponentEndOverlap`
  (params (OverlappedComponent :type "PrimitiveComponent Object Reference") (OtherActor :type "Actor Object Reference") (OtherComp :type "PrimitiveComponent Object Reference") (OtherBodyIndex :type Integer))
  (`AudioComponent.SetIntParameter` (`/Game/Blueprints/BP_AudioPlayer.Player` (`self.AudioPlayerReference`)) "SongValue" 0))

(fn `UserConstructionScript`)